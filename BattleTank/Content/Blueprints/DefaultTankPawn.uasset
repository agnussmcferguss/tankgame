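; DefaultTankPawn is a tank pawn Blueprint that handles look input for aiming the turret and barrel.
; HorizontalLook adds relative yaw to the Turret.
; VerticalLook adds the same axis value to SpringArm and Barrel pitch, clamping the barrel between MinPitch and MaxPitch and the camera arm to that range negated.
; The event graph and construction script are empty, and no movement or firing logic appears here.
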(event `InputAxis|HorizontalLook`
  (params (AxisValue :type "Float (single-precision)"))
  ;[1 1 1] Turn Turret (Yaw)
  (`SceneComponent.K2_AddRelativeRotation` (`self.Turret`) (`KismetMathLibrary.MakeRotator` 0.0 0.0 AxisValue) false false))

(event `InputAxis|VerticalLook`
  (params (AxisValue :type "Float (single-precision)"))
  (bind _maxpitch (`self.MaxPitch`))
  (bind _minpitch (`self.MinPitch`))
  (bind (_relativerotation_roll _relativerotation_pitch) (`KismetMathLibrary.BreakRotator` (`SceneComponent.RelativeRotation` (`self.Barrel`))))
  (bind (_relativerotation_roll_2 _relativerotation_pitch_2) (`KismetMathLibrary.BreakRotator` (`SceneComponent.RelativeRotation` (`self.SpringArm`))))
  ;[1 1 1] Move Camera (Pitch)
  (`SceneComponent.K2_SetRelativeRotation` (`self.SpringArm`) (`KismetMathLibrary.MakeRotator` 0.0 (`KismetMathLibrary.FClamp` (+ _relativerotation_pitch_2 AxisValue) (* _maxpitch -1.0) (* _minpitch -1.0))) false false)
  ;;[1 1 1] Set Barrel Pitch
  (`SceneComponent.K2_SetRelativeRotation` (`self.Barrel`) (`KismetMathLibrary.MakeRotator` 0.0 (`KismetMathLibrary.FClamp` (+ AxisValue _relativerotation_pitch) _minpitch _maxpitch)) false false))

(fn `UserConstructionScript`)